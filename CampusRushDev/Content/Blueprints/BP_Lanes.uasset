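; BP_Lanes is a trigger actor that supplies lane layout data to the runner.
; When a BP_Runner overlaps its Box, it copies the world locations of its center, left and right arrow components into the runner's lane position variables.
; It also passes its LanesAxis value to the runner, while other overlapping actors are ignored.
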(event OnComponentBeginOverlap(Box)
  (params (OverlappedComponent :type Primitive%20Component%20Object%20Reference) (OtherActor :type Actor%20Object%20Reference) (OtherComp :type Primitive%20Component%20Object%20Reference) (OtherBodyIndex :type Integer) (bFromSweep :type Boolean) (SweepResult :type Hit%20Result%20Structure%20%28by%20ref%29))
  (bind _asbp_runner (Utilities|Casting|CastToBP_Runner OtherActor))
  (Variables|/Game/Blueprints/BP_Runner.BP_Runner_C|SetCenterLanePosition _asbp_runner (Transformation|GetWorldLocation (Variables|Default|GetArrow)))
  (Variables|/Game/Blueprints/BP_Runner.BP_Runner_C|SetLeftLanePosition _asbp_runner (Transformation|GetWorldLocation (Variables|Default|GetArrowL)))
  (Variables|/Game/Blueprints/BP_Runner.BP_Runner_C|SetRightLanePosition _asbp_runner (Transformation|GetWorldLocation (Variables|Default|GetArrowR)))
  (Variables|/Game/Blueprints/BP_Runner.BP_Runner_C|SetLanesAxis _asbp_runner (Variables|Default|GetLanesAxis)))

(event EventBeginPlay)

(event Collision|EventActorBeginOverlap
  (params (OtherActor :type Actor%20Object%20Reference)))

(event EventTick
  (params (DeltaSeconds :type Float%20%28single-precision%29)))

(fn ConstructionScript)