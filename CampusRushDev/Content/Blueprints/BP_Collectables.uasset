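; BP_Collectables is an energy can pickup for the runner character.
; On BeginPlay a timeline spins the can mesh around yaw at a fixed tilt and replays itself whenever it finishes.
; When a BP_Runner overlaps it, the pickup adds a small amount to the runner's Energy and destroys itself.
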(event EventBeginPlay
  (bind _collectible_rotate (Timeline|CollectRotation Play)
    (:Update
      (Transformation|SetRelativeRotation (Variables|Default|GetSM_P_EnergyCan) (Math|Rotator|MakeRotator 3e+01 2.0 _collectible_rotate) false false))
    (:Finished
      (if true
        (Timeline|CollectRotation Play)))))

(event Collision|EventActorBeginOverlap
  (params (OtherActor :type Actor%20Object%20Reference))
  (bind _asbp_runner (Utilities|Casting|CastToBP_Runner OtherActor))
  (Variables|/Game/Blueprints/BP_Runner.BP_Runner_C|SetEnergy _asbp_runner (+ (Variables|/Game/Blueprints/BP_Runner.BP_Runner_C|GetEnergy _asbp_runner) 0.008))
  (Actor|DestroyActor))

(event EventTick
  (params (DeltaSeconds :type Float%20%28single-precision%29)))

(fn ConstructionScript)